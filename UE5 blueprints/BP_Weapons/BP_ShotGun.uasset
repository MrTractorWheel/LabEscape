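; BP_ShotGun is a shotgun weapon power-up pickup that upgrades the player's existing gun on overlap.
; When a BP_PlayerShooterCharacter overlaps it, it gets that character's gun and overwrites its damage and max range with the pickup's own values.
; It then prints acquisition messages and destroys itself, so the pickup is single-use and does not swap the gun actor.
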(event `self.ReceiveActorBeginOverlap`
  (params (OtherActor :type "Actor Object Reference"))
  (bind _asbp_player_shooter_character (cast `/Game/BP_Characters/BP_PlayerShooterCharacter` OtherActor))
  (bind _returnvalue (`ShooterCharacter.GetGun` _asbp_player_shooter_character))
  (`self.SetDamage` _returnvalue (`self.GetDamage` self))
  (`self.SetMaxRange` _returnvalue (`self.GetMaxRange` self))
  (`KismetSystemLibrary.PrintText` "Weapon damage increased!")
  (`KismetSystemLibrary.PrintText` "Shotgun Weapon-Power-Up Acquired!")
  (`self.K2_DestroyActor` self))

(fn `UserConstructionScript`)