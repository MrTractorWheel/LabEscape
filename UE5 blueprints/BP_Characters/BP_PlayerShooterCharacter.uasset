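; BP_PlayerShooterCharacter is the player shooter character Blueprint, whose only added logic here is pause menu toggling.
; A FlipFlop on the Pause input alternates between creating WBP_PauseMenu with the game paused and removing it to resume.
; Opening switches to game-and-UI input and shows the cursor, while closing restores game-only input without resetting the cursor flag.
; BeginPlay and the construction script only call their parents.
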(event `self.ReceiveBeginPlay`
  (`parent.ReceiveBeginPlay`))

(event `InputAction|Pause` :paused true
  (params (Key :type "Key Structure"))
  (bind _returnvalue (`GameplayStatics.GetPlayerController` 0))
  (:`Pressed`
    (`/Engine/EditorBlueprintResources/StandardMacros.FlipFlop`
      (:`A`
        (bind _returnvalue_2 (`|CreateWidget` "/Game/UI/WBP_PauseMenu.WBP_PauseMenu_C"))
        (`UserWidget.AddToViewport` _returnvalue_2 0)
        (`GameplayStatics.SetGamePaused` true)
        (`WidgetBlueprintLibrary.SetInputMode_GameAndUIEx` _returnvalue null)
        (set `PlayerController.bShowMouseCursor` true _returnvalue))
      (:`B`
        (`Widget.RemoveFromParent` _returnvalue_2)
        (`WidgetBlueprintLibrary.SetInputMode_GameOnly` (`GameplayStatics.GetPlayerController` 0))
        (`GameplayStatics.SetGamePaused` false)))))

(fn `UserConstructionScript`
  (`parent.UserConstructionScript`))